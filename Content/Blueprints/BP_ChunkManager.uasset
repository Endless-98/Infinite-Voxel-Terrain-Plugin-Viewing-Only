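; BP_ChunkManager starts voxel or chunk-based terrain generation for the selected world and applies the player's view-distance setting.
; On BeginPlay it loads the selected world name from a save slot, saving "DefaultWorld" if that fails, then sets the save name and initializes the terrain generator.
; Outside dedicated servers, it then loads saved quality settings and applies their chunk view distance as the generation radius.
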(event EventBeginPlay
  (bind _selectedworldsaveslot (Variables|Components|GetSelectedWorldSaveSlot))
  (Utilities|FlowControl|Sequence
    (:then_0
      (bind _returnvalue (SaveGame|DoesSaveGameExist _selectedworldsaveslot))
      (if _returnvalue
        (bind _returnvalue_2 (SaveGame|LoadGamefromSlot _selectedworldsaveslot))
        (bind _asbp_selected_world_save (Utilities|Casting|CastToBP_SelectedWorldSave _returnvalue_2)
          (:then
            (Variables|Components|SetSelected%20World%20Save (Variables|/InfiniteVoxelTerrainPlugin/Blueprints/Data/BP_SelectedWorldSave.BP_SelectedWorldSave_C|GetSelectedWorldSave _asbp_selected_world_save)))
          (:CastFailed
            (CallFunction|SaveSelectedName "DefaultWorld" :!label _label)))
        (else
          (goto _label)))
      (Class|ChunkManager|SetSaveGameName (Variables|Components|GetSelected%20World%20Save))
      (Class|ChunkManager|InitializeTerrainGenerator))
    (:then_1
      (if (not (Networking|IsDedicatedServer))
        (CallFunction|LoadQualitySettings)
        (CallFunction|ApplyQualitySettings)))))

(fn ConstructionScript)

(fn SaveSelectedName
  (params (SelectedWorldSave :type String))
  (bind _returnvalue (SaveGame|CreateSaveGameObject "/InfiniteVoxelTerrainPlugin/Blueprints/Data/BP_SelectedWorldSave.BP_SelectedWorldSave_C"))
  (bind _output_get (Variables|/InfiniteVoxelTerrainPlugin/Blueprints/Data/BP_SelectedWorldSave.BP_SelectedWorldSave_C|SetSelectedWorldSave _returnvalue SelectedWorldSave))
  (Variables|Components|SetSelected%20World%20Save _output_get)
  (bind _returnvalue_2 (SaveGame|SaveGametoSlot _returnvalue (LocalVariables|GetSelectedWorldSaveSlot)))
  (return _returnvalue_2))

(fn LoadQualitySettings
  (bind _qualitysettingssavename (Variables|Default|GetQualitySettingsSaveName))
  (bind _returnvalue (SaveGame|DoesSaveGameExist _qualitysettingssavename))
  (if _returnvalue
    (bind _returnvalue_2 (SaveGame|LoadGamefromSlot _qualitysettingssavename))
    (bind _asbp_quality_settings_save (Utilities|Casting|CastToBP_QualitySettingsSave _returnvalue_2)
      (:then
        (bind _output_get (Variables|Default|SetSettingsSaveObjectRef _asbp_quality_settings_save))
        (Variables|Components|SetQualitySettings (Variables|/InfiniteVoxelTerrainPlugin/Blueprints/Data/BP_QualitySettingsSave.BP_QualitySettingsSave_C|GetSavedQualitySettings _output_get))
        (return true))
      (:CastFailed
        (return false)))
    (else
      (return false))))

(fn ApplyQualitySettings
  (Class|ChunkManager|SetChunkGenerationRadius (.chunkviewdistance (Variables|Components|GetQualitySettings))))